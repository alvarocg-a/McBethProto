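; Interactable pickup actor that unlocks the second word text ("Palabra2") on the player character.
; Entering its Box trigger shows the "E to interact" prompt on the character's widget, and leaving hides it.
; The Interact event stores the interacting player and unhides that player's Palabra2 component.
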(event OnComponentBeginOverlap(Box)
  (params (OverlappedComponent :type Primitive%20Component%20Object%20Reference) (OtherActor :type Actor%20Object%20Reference) (OtherComp :type Primitive%20Component%20Object%20Reference) (OtherBodyIndex :type Integer) (bFromSweep :type Boolean) (SweepResult :type Hit%20Result%20Structure%20%28by%20ref%29))
  (bind _asbp_character (Utilities|Casting|CastToBP_Character OtherActor))
  (Variables|/Script/UMG.Widget|SetVisibility (Variables|/Game/McBethProto/UI/UI_Hud.UI_Hud_C|GetEtointeract (Variables|/Game/McBethProto/Core/BP_Character.BP_Character_C|GetWidget _asbp_character)) "Visible"))

(event OnComponentEndOverlap(Box)
  (params (OverlappedComponent :type Primitive%20Component%20Object%20Reference) (OtherActor :type Actor%20Object%20Reference) (OtherComp :type Primitive%20Component%20Object%20Reference) (OtherBodyIndex :type Integer))
  (bind _asbp_character (Utilities|Casting|CastToBP_Character OtherActor))
  (Variables|/Script/UMG.Widget|SetVisibility (Variables|/Game/McBethProto/UI/UI_Hud.UI_Hud_C|GetEtointeract (Variables|/Game/McBethProto/Core/BP_Character.BP_Character_C|GetWidget _asbp_character)) "Hidden"))

(event EventBeginPlay
  (|CallParentFunction) ; This node is disabled and will not be called.\nDrag off pins to build functionality.
)

(event Collision|EventActorBeginOverlap
  (params (OtherActor :type Actor%20Object%20Reference)))

(event EventTick
  (params (DeltaSeconds :type Float%20%28single-precision%29)))

(event EventInteract
  (params (Player :type BP%20Character%20Object%20Reference))
  (bind _output_get (Variables|Default|SetPlayer Player))
  (Development|SetHiddeninGame (Variables|/Game/McBethProto/Core/BP_Character.BP_Character_C|GetPalabra%202 _output_get) false false))

(fn ConstructionScript
  (|CallParentFunction))
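; BP_BloqueoParent is a parent Blueprint for blockers that the player clears by interacting, using a matching key if locked.
; Interact searches the player's Inventary for a BP_Key whose DesbloqueoRef matches TipoDeBloqueo, breaking the loop through a custom event on a match.
; A match overwrites NoKeyMessage with the used type, and that variable is printed after the search.
; InteractSucces, called on a match or when unlocked, destroys the actor.
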(event Custom|BreakeLoopInventaryCheck
  (Utilities|Array|ForEachLoopwithBreak (Variables|/Game/McBethProto/Core/BP_Character.BP_Character_C|GetInventary (stale EventInteract Player))) ; enters at Break
)

(event EventBeginPlay
  (|CallParentFunction))

(event EventInteractSucces
  (Actor|DestroyActor))

(event EventInteract
  (params (Player :type BP%20Character%20Object%20Reference))
  (if (Variables|Default|GetIsLocked)
    (bind _array_element (Utilities|Array|ForEachLoopwithBreak (Variables|/Game/McBethProto/Core/BP_Character.BP_Character_C|GetInventary Player))
      (:LoopBody
        (bind _asbp_key (Utilities|Casting|CastToBP_Key _array_element))
        (if (Utilities|Enum|Equal(Enum) (Variables|/Game/McBethProto/Blueprints/Pickeable/Keys/BP_Key.BP_Key_C|GetDesbloqueoRef _asbp_key) (Variables|Default|GetTipo%20de%20Bloqueo))
          (Variables|Default|SetNoKeyMessage (Utilities|String|Append "Has usado " (Utilities|String|EnumtoString (Variables|Default|GetTipo%20de%20Bloqueo))))
          (CallFunction|BreakeLoopInventaryCheck)
          (CallFunction|InteractSucces)))
      (:Completed
        (Development|PrintString (Variables|Default|GetNoKeyMessage))))
    (else
      (CallFunction|InteractSucces))))

(fn ConstructionScript
  (|CallParentFunction))
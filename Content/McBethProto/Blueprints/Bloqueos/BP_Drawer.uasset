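; BP_Drawer is an interactable drawer that opens and closes on successful interaction.
; On BeginPlay it attaches up to two optional content references to billboard components, snapping location while keeping relative rotation and world scale.
; Each InteractSucces flips between playing and reversing the OpendClose timeline, which lerps the Cube's relative location from zero to the EndAnimationPos component's position.
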(event EventBeginPlay
  (|CallParentFunction)
  (bind _drawercontent_1 (Variables|Default|GetDrawerContent_1)
    (:then
      (Transformation|AttachComponentToComponent _drawercontent_1 (Variables|Default|GetBillboard) "None" "SnapToTarget" "KeepRelative" "KeepWorld" true))
    (:else
      _))
  (bind _drawercontent_2 (Variables|Default|GetDrawerContent_2)
    (:then
      (Transformation|AttachComponentToComponent _drawercontent_2 (Variables|Default|GetBillboard1) "None" "SnapToTarget" "KeepRelative" "KeepWorld" true))
    (:else)))

(event EventInteractSucces
  (Utilities|FlowControl|FlipFlop
    (:A
      (bind _newtrack_0 (Timeline|Opend/Close Play)
        (:Update
          (Transformation|SetRelativeLocation (Variables|Default|GetCube) (Math|Vector|Lerp(Vector) "0, 0, 0" (Variables|/Script/Engine.SceneComponent|GetRelativeLocation (Variables|Default|GetEndAnimationPos)) _newtrack_0) false false))))
    (:B
      (Timeline|Opend/Close Reverse))))

(fn ConstructionScript
  (|CallParentFunction))
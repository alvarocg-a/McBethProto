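; BP_ClosedDoor is an interactable door that moves and triggers a one-time collapse that reveals rubble.
; Each successful interaction alternates a timeline forward and backward, lerping the Cube's relative location between zero and the EndAnimationPos component's location.
; The first timeline update unhides the valid Escombros actors, enables their collision and plays a collapse sound once at world origin.
; Reversing the door leaves the rubble in place.
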(event EventBeginPlay
  (|CallParentFunction) ; This node is disabled and will not be called.\nDrag off pins to build functionality.
)

(event EventInteractSucces
  (Utilities|FlowControl|FlipFlop
    (:A
      (bind _newtrack_0 (Timeline|Timeline Play)
        (:Update
          (Transformation|SetRelativeLocationAndRotation (Variables|Default|GetCube) (Math|Vector|Lerp(Vector) "0, 0, 0" (Variables|/Script/Engine.SceneComponent|GetRelativeLocation (Variables|Default|GetEndAnimationPos)) _newtrack_0) "0, 0, 0" false false)
          (Utilities|FlowControl|DoOnce false
            (:Completed
              (for _array_element (Variables|Default|GetEscombros)
                (Utilities|IsValid _array_element
                  (:Is%20Valid
                    (Rendering|SetActorHiddenInGame _array_element false)
                    (Collision|SetActorEnableCollision _array_element true)
                    (Utilities|FlowControl|DoOnce false
                      (:Completed
                        (Audio|PlaySoundatLocation "/Game/StarterContent/Audio/Collapse01.Collapse01" "0, 0, 0" "0, 0, 0" 1.0 1.0 0.0 0 0 0 0)))))))))))
    (:B
      (Timeline|Timeline Reverse))))

(fn ConstructionScript
  (|CallParentFunction))
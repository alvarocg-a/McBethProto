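; BP_MemoryParent is a base Blueprint for interactable memories that play a dialogue line.
; BeginPlay assigns DialogueLine to the Audio component, and Interact plays it.
; A DoOnce boolean selects between a single playback and a repeatable one, whose gate resets after the line's duration so replays cannot overlap.
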(event EventBeginPlay
  (|CallParentFunction)
  (Audio|Components|Audio|SetSound (Variables|Default|GetAudio) (Variables|Default|GetDialogueLine)))

(event EventInteract
  (params (Player :type BP%20Character%20Object%20Reference))
  (if (Variables|Default|GetdoOnce)
    (Utilities|FlowControl|DoOnce false
      (:Completed
        (Audio|Components|Audio|Play (Variables|Default|GetAudio) 0.0)))
    (else
      (Utilities|FlowControl|DoOnce false :!label _label
        (:Completed
          (Audio|Components|Audio|Play (Variables|Default|GetAudio) 0.0)
          (Utilities|FlowControl|Delay (Variables|/Script/Engine.SoundBase|GetDuration (Variables|Default|GetDialogueLine)))
          (goto _label Reset))))))

(fn ConstructionScript
  (|CallParentFunction))
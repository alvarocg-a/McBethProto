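; Lady Macbeth NPC that gates a chained letter, candle and note puzzle, answering interactions with Spanish debug-print lines.
; Interact takes the player's letter to grant a candle, then spawns the final note once the candle and note flags are set.
; MoveToNextTorch walks her via AI through lit torches in array order, then sets the candle flag and opens an empty drawer.
; The note flag is only read here.
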(event Custom|MoveToNextTorch
  (bind _torches (Variables|Default|GetTorches))
  (bind _torchindex (Variables|Default|GetTorchIndex))
  (bind _output (Utilities|Array|Get(acopy) _torches _torchindex))
  (Utilities|FlowControl|Delay 0.6)
  (if (Variables|/Game/McBethProto/Blueprints/BP_Torch.BP_Torch_C|GetIsLighted _output)
    (AI|AIMoveTo (AI|GetAIController self) "0, 0, 0" _output -1.0 "Default" "Default" true true
      (:OnMoveFinished
        (bind _result (Math|Integer|IncrementInt (Variables|Default|GetTorchIndex))
          (:%20%20
            (if (> _result (- (Utilities|Array|Length (Variables|Default|GetTorches)) 1))
              (Variables|Default|SetPuzzle_Canlde true)
              (Utilities|FlowControl|Delay 0.2)
              (Development|PrintString "Escribir, debo escribir.")
              (Default|OpenDrawer (Variables|Default|GetDrawerEmpty))
              (Development|PrintString "No esta, donde esta")
              (else
                (CallFunction|MovetoNextTorch)))))))))

(event Custom|Interact
  (params (Player :type BP%20Character%20Object%20Reference))
  (Variables|Default|SetPlayer Player)
  (if (Variables|Default|GetPuzzle_Letter)
    (if (Variables|Default|GetPuzzle_Canlde)
      (if (Variables|Default|GetPuzzle_Note)
        (Development|PrintString "ahora puedo escribir")
        (Utilities|FlowControl|Delay 1.0)
        (Game|SpawnActorfromClass "/Game/McBethProto/Blueprints/Pickeable/BP_NoteFinal.BP_NoteFinal_C" (Transformation|GetActorTransform (Variables|Default|GetNotaSpawnPoint)) "Undefined" "MultiplyWithRoot" 0 0)
        (else
          (Development|PrintString "Necesito escribir, escribir, algo para escribir, estaba aqui, donde??")))
      (else
        (Development|PrintString "Odio la oscuridad, no ire si no hay luz")))
    (elif (Variables|/Game/McBethProto/Core/BP_Character.BP_Character_C|GetHas_Letter (Variables|Default|GetPlayer))
      (Variables|Default|SetPuzzle_Letter true)
      (Development|PrintString "Has completado el puzzle, toma una velita, para tu")
      (Variables|/Game/McBethProto/Core/BP_Character.BP_Character_C|SetHas_Candle (Variables|Default|GetPlayer) true)
      (else
        (Development|PrintString "traeme mi carta")))))

(fn ConstructionScript)
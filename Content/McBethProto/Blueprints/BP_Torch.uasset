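; BP_Torch is an interactable torch that the player lights with a candle to advance Lady Macbeth.
; Interact checks that the player has a candle, then passes through a DoOnce so the torch lights only once.
; Lighting unhides the point light, flags the torch as lit and tells the player's LadyMacbeth reference to move to the next torch.
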(event Custom|Ligth
  (Development|SetHiddeninGame (Variables|Default|GetPointLight) false false)
  (Variables|Default|SetIsLighted true)
  (Default|MovetoNextTorch (Variables|/Game/McBethProto/Core/BP_Character.BP_Character_C|GetLadyMacbeth (stale EventInteract Player))))

(event EventBeginPlay
  (|CallParentFunction))

(event EventInteract
  (params (Player :type BP%20Character%20Object%20Reference))
  (if (Variables|/Game/McBethProto/Core/BP_Character.BP_Character_C|GetHas_Candle Player)
    (Utilities|FlowControl|DoOnce false
      (:Completed
        (CallFunction|Ligth)))))

(fn ConstructionScript
  (|CallParentFunction))
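; BP_LetterFragment is a pickeable letter fragment the player collects through an Interact event.
; After the parent interaction runs, it filters the player's Inventary for fragments and compares that count with all fragment actors in the level.
; When the counts match, it sets HasLetter on the player and prints a Spanish completion message; otherwise it prints the note name with an added-to-inventory message.
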(event EventBeginPlay
  (|CallParentFunction) ; This node is disabled and will not be called.\nDrag off pins to build functionality.
)

(event Collision|EventActorBeginOverlap
  (params (OtherActor :type Actor%20Object%20Reference)))

(event EventTick
  (params (DeltaSeconds :type Float%20%28single-precision%29)))

(event EventInteract
  (params (Player :type BP%20Character%20Object%20Reference))
  (|CallParentFunction Player)
  (bind _filteredarray (Utilities|Array|FilterArray (Variables|/Game/McBethProto/Core/BP_Character.BP_Character_C|GetInventary Player) "BP_LetterFragment_C"))
  (bind _outactors (Actor|GetAllActorsOfClass "BP_LetterFragment_C"))
  (if (== (Utilities|Array|Length _outactors) (Utilities|Array|Length _filteredarray))
    (Development|PrintString "Ya tienes todos los fragmentos")
    (Variables|/Game/McBethProto/Core/BP_Character.BP_Character_C|SetHas_Letter Player true)
    (else
      (Development|PrintString (Utilities|String|Append (Variables|Default|GetNoteName) " Se ha añadido a tu inventario")))))

(fn ConstructionScript
  (|CallParentFunction))
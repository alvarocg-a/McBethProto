(event EventBeginPlay
  (|CallParentFunction) ; This node is disabled and will not be called.\nDrag off pins to build functionality.
)

(event EventInteract
  (params (Player :type BP%20Character%20Object%20Reference))
  (Utilities|Array|Add (Variables|/Game/McBethProto/Core/BP_Character.BP_Character_C|GetInventary Player) self)
  (Rendering|SetActorHiddenInGame true)
  (Collision|SetActorEnableCollision false)
  (Development|PrintString (Utilities|String|Append (Utilities|String|EnumtoString (Variables|Default|GetDesbloqueoRef)) " Se ha añadido a tu inventario")))

(fn ConstructionScript
  (|CallParentFunction))
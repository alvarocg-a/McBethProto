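; Base physical object for a past/present timeline-switching mechanic, where moving it in the past changes its position in the present.
; On each timeline change it saves the cube's transform for the timeline being left and restores the other.
; A BP_Character hit in the past flags a change, so returning to the present keeps the past position.
; That hit also prints a Spanish notice once per visit to the past.
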(event OnComponentHit(Cube)
  (params (HitComponent :type Primitive%20Component%20Object%20Reference) (OtherActor :type Actor%20Object%20Reference) (OtherComp :type Primitive%20Component%20Object%20Reference) (NormalImpulse :type Vector :default "0, 0, 0") (Hit :type Hit%20Result%20Structure%20%28by%20ref%29))
  (Utilities|Casting|CastToBP_Character OtherActor)
  (if (Variables|Default|GetIs%20Past)
    (Variables|Default|SetChangedPast true)
    (Utilities|FlowControl|DoOnce false
      (:Completed
        (Development|PrintString "Has movido un objeto en el pasado 
El objeto en el presente cambiara de lugar")))))

(event EventBeginPlay
  (Variables|Default|SetPresentTransform (Transformation|GetWorldTransform (Variables|Default|GetCube)))
  (|CallParentFunction))

(event EventChangeTimelineEvent
  (params (IsPast :type Boolean))
  (if IsPast
    (Variables|Default|SetPresentTransform (Transformation|GetWorldTransform (Variables|Default|GetCube)))
    (Transformation|SetWorldTransform (Variables|Default|GetCube) (Variables|Default|GetPastTransform) false false)
    (Variables|Default|SetChangedPast false)
    (Utilities|FlowControl|DoOnce false) ; enters at Reset
    (else
      (Variables|Default|SetPastTransform (Transformation|GetWorldTransform (Variables|Default|GetCube)))
      (if (not (Variables|Default|GetChangedPast))
        (Transformation|SetWorldTransform (Variables|Default|GetCube) (Variables|Default|GetPresentTransform) false false)))))

(fn ConstructionScript
  (|CallParentFunction))
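; Parent NPC interactable for a word-collecting prototype, where the player talks to an NPC in Spanish dialogue about remembering and names.
; Box overlap toggles the interact prompt on the BP_Character widget and recolors the player's Palabra1 word, if visible, as usable or normal.
; Interact, marked as a non-final test, opens the word UI with mouse input when HasAllWords is set.
; Otherwise TalkedBefore and Palabra1's visibility choose the dialogue and objective update.
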(event OnComponentBeginOverlap(Box)
  (params (OverlappedComponent :type Primitive%20Component%20Object%20Reference) (OtherActor :type Actor%20Object%20Reference) (OtherComp :type Primitive%20Component%20Object%20Reference) (OtherBodyIndex :type Integer) (bFromSweep :type Boolean) (SweepResult :type Hit%20Result%20Structure%20%28by%20ref%29))
  ;[1 1 1] ACtivar UI Prompt
  (bind _asbp_character (Utilities|Casting|CastToBP_Character OtherActor))
  (Variables|/Game/McBethProto/UI/UI_Hud.UI_Hud_C|SetVisibility_0 (Variables|/Game/McBethProto/Core/BP_Character.BP_Character_C|GetWidget _asbp_character) "Visible")
  (if (not (Variables|/Script/Engine.SceneComponent|GetbHiddenInGame (Variables|/Game/McBethProto/Core/BP_Character.BP_Character_C|GetPalabra%201 _asbp_character)))
    (Rendering|Components|TextRender|SetTextRenderColor (Variables|/Game/McBethProto/Core/BP_Character.BP_Character_C|GetPalabra%201 _asbp_character) (Variables|Default|GetUsable))))

(event OnComponentEndOverlap(Box)
  (params (OverlappedComponent :type Primitive%20Component%20Object%20Reference) (OtherActor :type Actor%20Object%20Reference) (OtherComp :type Primitive%20Component%20Object%20Reference) (OtherBodyIndex :type Integer))
  ;[1 1 1] ACtivar UI Prompt
  (bind _asbp_character (Utilities|Casting|CastToBP_Character OtherActor))
  (Variables|/Script/UMG.Widget|SetVisibility (Variables|/Game/McBethProto/UI/UI_Hud.UI_Hud_C|GetEtointeract (Variables|/Game/McBethProto/Core/BP_Character.BP_Character_C|GetWidget _asbp_character)) "Hidden")
  (Variables|/Script/UMG.TextBlock|SetText (Variables|/Game/McBethProto/UI/UI_Hud.UI_Hud_C|GetEtointeract (Variables|/Game/McBethProto/Core/BP_Character.BP_Character_C|GetWidget _asbp_character)) "Press F to interact")
  (if (not (Variables|/Script/Engine.SceneComponent|GetbHiddenInGame (Variables|/Game/McBethProto/Core/BP_Character.BP_Character_C|GetPalabra%201 (stale OnComponentBeginOverlap(Box) _asbp_character))))
    (Rendering|Components|TextRender|SetTextRenderColor (Variables|/Game/McBethProto/Core/BP_Character.BP_Character_C|GetPalabra%201 (stale OnComponentBeginOverlap(Box) _asbp_character)) (Variables|Default|GetNormal))))

(event EventBeginPlay
  (|CallParentFunction) ; This node is disabled and will not be called.\nDrag off pins to build functionality.
)

(event Collision|EventActorBeginOverlap
  (params (OtherActor :type Actor%20Object%20Reference)))

(event EventTick
  (params (DeltaSeconds :type Float%20%28single-precision%29)))

(event EventInteract
  (params (Player :type BP%20Character%20Object%20Reference))
  (bind _returnvalue (Game|GetPlayerController 0))
  (bind _widget (Variables|/Game/McBethProto/Core/BP_Character.BP_Character_C|GetWidget Player))
  (bind _etointeract (Variables|/Game/McBethProto/UI/UI_Hud.UI_Hud_C|GetEtointeract _widget))
  ;[1 1 1] Interact - Test no FINAL no tocar
  (if (Variables|Default|GetHas%20all%20Words)
    (Input|SetInputModeUIOnly _returnvalue _widget "DoNotLock" false)
    (Variables|/Game/McBethProto/UI/UI_Hud.UI_Hud_C|SetVisibility_Words _widget "Visible")
    (Variables|/Script/Engine.PlayerController|SetbShowMouseCursor _returnvalue true)
    (Variables|/Game/McBethProto/UI/UI_Hud.UI_Hud_C|SetVisibility_0 _widget "Hidden")
    (elif (Variables|Default|GetTalkedBefore)
      (if (Variables|/Script/Engine.SceneComponent|GetbHiddenInGame (Variables|/Game/McBethProto/Core/BP_Character.BP_Character_C|GetPalabra%201 Player))
        (Variables|/Script/UMG.TextBlock|SetText _etointeract "Si los ojos son la puerta del alma El nombre es la LLAVE")
        (else
          (Variables|/Script/UMG.TextBlock|SetText _etointeract "Como sabias mi Nombre? Claro que me gusta el pan")
          (Utilities|FlowControl|Delay 3.0)
          (Variables|/Script/UMG.TextBlock|SetText _etointeract "Donde estoy, QUE ESTA PASANDO?? Necesito ayuda")
          (Variables|/Script/UMG.TextBlock|SetText (Variables|/Game/McBethProto/UI/UI_Hud.UI_Hud_C|GetObjetivos _widget) "Busca mas Palabras")
          (Variables|Default|SetTalkedBefore false)))
      (else
        (Variables|/Script/UMG.TextBlock|SetText _etointeract "Porfavor Ayudame a Recordar")))))

(fn ConstructionScript
  (|CallParentFunction))